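; Enemy AI pawn that chases the player on sight and knocks characters into the air with a melee attack.
; Pawn Sensing triggers the chase, which uses AI MoveTo toward the player and, on arrival, plays an attack montage gated by the Attack flag.
; As the montage starts, a forward sphere trace launches any hit character and plays a 3D sound; montage completion or interruption re-arms the attack.
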(event OnSeePawn(PawnSensing)
  (params (Pawn :type Pawn%20Object%20Reference))
  ;[0.05098 0.05098 0.05098] AI Function
  (CallFunction|AIChase))

(event Custom|AI_Chase
  (bind _sphere (Variables|Default|GetSphere))
  (bind _returnvalue (Transformation|GetSocketLocation _sphere "None"))
  ;[0.05098 0.05098 0.05098] Chase Input
  (AI|AIMoveTo self "0, 0, 0" (Game|GetPlayerCharacter 0) 1.2e+02 false
    (:OnSuccess
      (if (Variables|Default|GetAttack?)
        (Animation|Montage|PlayMontage (Variables|Character|GetMesh) "/Game/Characters/Monster/Source/Animations/M_M_attack.M_M_attack"
          (:then
            (Variables|Default|SetAttack? false)
            (bind (_outhit _returnvalue_2) (Collision|SphereTraceByChannel _returnvalue (+ _returnvalue (* (Math|Vector|GetForwardVector (Transformation|GetActorRotation)) 2e+02)) 25.0 "TraceTypeQuery3" false 0 "None" true "(R=1.000000,G=0.000000,B=0.000000,A=1.000000)" "(R=0.000000,G=1.000000,B=0.000000,A=1.000000)" 0.5))
            (if _returnvalue_2
              (bind _ascharacter (Utilities|Casting|CastToCharacter (.HitActor (Collision|BreakHitResult _outhit))))
              (Character|LaunchCharacter _ascharacter (+ (* (Math|Vector|GetForwardVector (Transformation|GetActorRotation)) 8.5e+02) "0.000000,0.000000,1000.000000") false false)
              (Audio|PlaySoundatLocation "/Game/Audio/MS_OOF.MS_OOF" (Transformation|GetActorLocation) "0, 0, 0" 1.0 1.0 0.0 "/Game/Audio/Audio_3D.Audio_3D" 0 0 0)))
          (:OnCompleted
            (Variables|Default|SetAttack? true :!label _label))
          (:OnInterrupted
            (goto _label)))))))

(event EventBeginPlay
  (Variables|Default|SetHealth 50))

(event Collision|EventActorBeginOverlap
  (params (OtherActor :type Actor%20Object%20Reference)))

(event EventTick
  (params (DeltaSeconds :type Float%20%28single-precision%29)))

(fn ConstructionScript)